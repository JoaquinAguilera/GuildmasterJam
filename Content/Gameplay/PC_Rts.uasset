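; PC_Rts is an RTS player controller that feeds left-mouse marquee input to the HUD.
; On BeginPlay it shows the cursor and sets Game and UI input with the mouse always locked to the window.
; Mouse press and release set a held flag and send marquee messages to the HUD, while Tick sends a held message until release.
; A TODO marks this polling for replacement with Enhanced Input.
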(event `self.ReceiveBeginPlay`
  ;[0 0 0] Set lock window, show cursor
  (`WidgetBlueprintLibrary.SetInputMode_GameAndUIEx` self null "LockAlways" false)
  (set `self.bShowMouseCursor` true))

(event `Key|LeftMouseButton`
  (params (Key :type "Key Structure"))
  (bind _returnvalue (`self.GetHUD`))
  ;[1 0 0] TODO: Replace with enhanced input held
  (:`Pressed`
    (set `self.IsLeftMousePressed` true)
    (message `/Game/Gameplay/BIF_RTS.MarqueePressed` _returnvalue))
  (:`Released`
    (set `self.IsLeftMousePressed` false)
    (message `/Game/Gameplay/BIF_RTS.MarqueeReleased` _returnvalue)))

(event `self.ReceiveTick`
  (params (DeltaSeconds :type "Float (single-precision)"))
  (if (`self.IsLeftMousePressed`)
    (message `/Game/Gameplay/BIF_RTS.MarqueeHeld` (`self.GetHUD`))))

(fn `UserConstructionScript`)