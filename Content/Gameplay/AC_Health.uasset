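; Health component that tracks current health and death state for its owning actor, starting from max health on BeginPlay.
; ChangeHealth applies signed amounts while alive, caps only at the maximum, and triggers DeathEvent at zero or below.
; DeathEvent sets the dead flag and calls the OnDeath dispatcher.
; Debug keys add or remove health, with on-screen prints reporting health and death.
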(event Custom|DeathEvent
  ;[0 0 0] Death Event
  (Variables|ACHealth|SetIsDead true)
  (Default|CallOnDeath)
  (Development|PrintString (Utilities|String|Append (Utilities|GetDisplayName (Components|GetOwner)) " has died.") true true "(R=1.000000,G=0.000000,B=0.000000,A=1.000000)" 8.0))

(event EventBeginPlay
  ;[0 0 0] Initialize
  (CallFunction|ChangeHealth (Variables|Settings|GetMaxHealth)))

(event Input|KeyboardEvents|DebugKeyS
  (params (Key :type Key%20Structure :default "None") (ActionValue :type Input%20Action%20Value%20Structure))
  ;[1 0 0] Debug health add/remove
  (:Pressed
    (CallFunction|ChangeHealth -2e+01)
    (Development|PrintString (Utilities|String|ToString(Float) (Variables|ACHealth|GetCurrentHealth)))))

(event Input|KeyboardEvents|DebugKeyE
  (params (Key :type Key%20Structure :default "None") (ActionValue :type Input%20Action%20Value%20Structure))
  ;[1 0 0] Debug health add/remove
  (:Pressed
    (CallFunction|ChangeHealth 2e+01)
    (Development|PrintString (Utilities|String|ToString(Float) (Variables|ACHealth|GetCurrentHealth)))))

(fn ChangeHealth
  (params (Amount :type Float%20%28double-precision%29))
  (Utilities|FlowControl|Sequence
    (:then_0
      (LocalVariables|SetHealthChangeValue Amount)
      (if (not (Variables|ACHealth|GetIsDead))
        (if (>= (Variables|Settings|GetMaxHealth) (+ (Variables|ACHealth|GetCurrentHealth) (LocalVariables|GetHealthChangeValue)))
          (bind _output_get (Variables|ACHealth|SetCurrentHealth (+ (Variables|ACHealth|GetCurrentHealth) (LocalVariables|GetHealthChangeValue))))
          (else
            (Variables|ACHealth|SetCurrentHealth (Variables|Settings|GetMaxHealth)) ; Max Health Reached, set to max instead
          ))
        (if (<= _output_get 0.0) ; Is Dead, Set Dead
          (CallFunction|DeathEvent))))
    (:then_1
      (Development|PrintString (Utilities|String|Append "Current Health on:  " (Utilities|GetDisplayName (Components|GetOwner)) " = " (Utilities|String|ToString(Float) (Variables|ACHealth|GetCurrentHealth))) true true "(R=0.000000,G=0.660000,B=1.000000,A=1.000000)" 5.0))))